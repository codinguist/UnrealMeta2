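; Blueprint that slides its StaticMesh back and forth along its relative X axis, starting automatically at BeginPlay.
; A timeline's value, scaled to a fixed distance, sets the mesh's relative location on each update.
; The IsMoveRight flag selects Play or Reverse, and each Finished event flips it and re-enters the branch for an endless ping-pong.
; An EnableInput call is present but never runs.
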(event `self.ReceiveBeginPlay`
  (if (`self.is Move Right`) :!label _label
    (bind (_direction _value) (`Timeline|타임라인_0` :!label _label_2)
      (:`Update`
        (`SceneComponent.K2_SetRelativeLocation` (`self.StaticMesh`) (`KismetMathLibrary.MakeVector` (* _value 1000.0)) false false))
      (:`Finished`
        (set `self.is Move Right` (not (`self.is Move Right`)))
        (goto _label)))
    (else
      (goto _label_2 :!via `Reverse`))))

(fn `UserConstructionScript`)